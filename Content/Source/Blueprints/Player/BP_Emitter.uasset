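; Player wave emitter that fires waves in one of three colours from a pitch-clamped rotatable dish.
; A looping timer spawns a wave at the Scene transform and applies the material for the current colour index.
; Colour inputs cycle the index, creating a new HUD widget only on wrap; ColourUp's wrap loops back and increments again.
; Tick calls the game state's FailState every frame.
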(event EventTick
  (params (DeltaSeconds :type Float%20%28single-precision%29))
  (bind _asbp_game_state (Utilities|Casting|CastToBP_GameState (Game|GetGameState)))
  (Default|FailState _asbp_game_state))

(event EventBeginPlay
  (Utilities|Time|SetTimerbyFunctionName 0 "SpawnWave" (/ (/ 128.0 6e+01) 15.0) true))

(event Input|ActionEvents|InputActionColourUp
  (params (Key :type Key%20Structure))
  (:Pressed
    (if (> (+ (Variables|Default|GetWaveColourIndex) 1) 2) :!label _label
      (bind _output_get (Variables|Default|SetWaveColourIndex 0))
      (bind _returnvalue (UserInterface|CreateWidget "/Game/Source/UI/HUD/Widget_HUD.Widget_HUD_C" (Game|GetPlayerController 0)))
      (bind _output_get_2 (Variables|Default|SetHUDRef _returnvalue))
      (Default|SwitchColor _output_get_2 _output_get)
      (goto _label)
      (else
        (Variables|Default|SetWaveColourIndex (+ (Variables|Default|GetWaveColourIndex) 1))))))

(event Input|ActionEvents|InputActionColourDown
  (params (Key :type Key%20Structure))
  (:Pressed
    (if (< (- (Variables|Default|GetWaveColourIndex) 1) 0)
      (bind _output_get (Variables|Default|SetWaveColourIndex 2))
      (bind _returnvalue (UserInterface|CreateWidget "/Game/Source/UI/HUD/Widget_HUD.Widget_HUD_C" (Game|GetPlayerController 0)))
      (bind _output_get_2 (Variables|Default|SetHUDRef _returnvalue))
      (Default|SwitchColor _output_get_2 _output_get)
      (else
        (Variables|Default|SetWaveColourIndex (- (Variables|Default|GetWaveColourIndex) 1))))))

(event Input|AxisEvents|InputAxisEmitterMovement
  (params (AxisValue :type Float%20%28single-precision%29))
  (bind _dishsprite (Variables|Default|GetDishSprite))
  (bind _returnvalue (Transformation|GetWorldRotation _dishsprite))
  (Transformation|SetWorldRotation (Variables|Default|GetDishSprite) (Math|Rotator|MakeRotator (.roll _returnvalue) (Math|Float|Clamp(Float) (+ AxisValue (.pitch _returnvalue)) -6e+01 6e+01) (.yaw _returnvalue)) false false))

(fn ConstructionScript)

(fn SpawnWave
  (bind _returnvalue (Game|SpawnActorfromClass (Variables|Default|GetWaveClass) (Transformation|GetWorldTransform (Variables|Default|GetScene)) "AlwaysSpawn" 0 0))
  (Utilities|IsValid _returnvalue
    (:Is%20Valid
      (Rendering|Material|SetMaterial (Variables|/Game/Source/Blueprints/Projectiles/BP_Wave.BP_Wave_C|GetPlane _returnvalue) 0 (Utilities|Array|Get(acopy) (Variables|Default|GetWaveMaterials) (Variables|Default|GetWaveColourIndex))))))