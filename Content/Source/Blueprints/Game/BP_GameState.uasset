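; BP_GameState is the game state that drives the Work drain, game time and game-over condition.
; A looping timer from BeginPlay calls DecreaseWork on the first player's BP_PlayerState until EndPlay clears it, while Tick accumulates GameTime.
; FailState, not called within this Blueprint, checks whether Work equals MinWork, then pauses the game and shows the game-over widget with UI-only input.
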(event Custom|DecreaseWork
  (bind _asbp_game_state (Utilities|Casting|CastToBP_GameState (Game|GetGameState)))
  (bind _asbp_player_state (Utilities|Casting|CastToBP_PlayerState (Utilities|Array|Get(acopy) (Variables|/Script/Engine.GameStateBase|GetPlayerArray _asbp_game_state))))
  (Default|DecreaseWork _asbp_player_state))

(event Custom|FailState
  (bind _returnvalue (Game|GetPlayerController 0))
  (bind _asbp_player_state (Utilities|Casting|CastToBP_PlayerState (Utilities|Array|Get(acopy) (Variables|Default|GetPlayerArray))))
  (if (== (Variables|/Game/Source/Blueprints/Game/BP_PlayerState.BP_PlayerState_C|GetWork _asbp_player_state) (Variables|/Game/Source/Blueprints/Game/BP_PlayerState.BP_PlayerState_C|GetMinWork _asbp_player_state))
    (Game|SetGamePaused true)
    (bind _returnvalue_2 (UserInterface|CreateWidget "/Game/Source/UI/Menu/Widget_GameOver.Widget_GameOver_C" _returnvalue))
    (UserInterface|Viewport|AddtoViewport _returnvalue_2 0)
    (Variables|/Script/Engine.PlayerController|SetbShowMouseCursor _returnvalue true)
    (Input|SetInputModeUIOnly _returnvalue _returnvalue_2 "DoNotLock")))

(event EventTick
  (params (DeltaSeconds :type Float%20%28single-precision%29))
  (Variables|Default|SetGameTime (+ DeltaSeconds (Variables|Default|GetGameTime))))

(event EventBeginPlay
  (bind _returnvalue (Utilities|Time|SetTimerbyFunctionName 0 "DecreaseWork" 0.1 true))
  (Variables|Default|SetTempHandle _returnvalue))

(event EventEndPlay
  (params (EndPlayReason :type EEndPlayReason%20Enum :default "Destroyed"))
  (Utilities|Time|ClearandInvalidateTimerbyHandle (Variables|Default|GetTempHandle)))

(fn ConstructionScript)