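; BP_Bat is a flipbook bat pawn that follows a spline while happy and otherwise flies to a fixed roost to hang.
; A looping timer drains its happiness after a startup delay, and overlaps with BP_Wave raise it.
; SetBatState, not called within this Blueprint, maps happiness to a status enum and the IsHappy flag.
; Tick reads that flag to steer via FloatingPawnMovement and choose flipbooks.
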(event EventBeginPlay
  (Utilities|FlowControl|Sequence
    (:then_0
      (Utilities|FlowControl|Delay 5.0)
      (Utilities|Time|SetTimerbyFunctionName 0 "DecrementBatState" 0.1 true))
    (:then_1
      (Variables|Default|SetSpline%20Dist 0.0)
      (Transformation|SetWorldLocation (Variables|Default|GetDummyRoot) (Spline|GetLocationatDistanceAlongSpline (Variables|/Game/BP_FigureEightSpline.BP_FigureEightSpline_C|GetSpline (Variables|Default|GetSplineBP)) (Variables|Default|GetSpline%20Dist) "World") false false))))

(event EventTick
  (params (DeltaSeconds :type Float%20%28single-precision%29))
  (bind _returnvalue (Transformation|GetActorLocation))
  (bind _returnvalue_2 (Math|Vector|MakeVector 1.65e+03 3.6e+02 -4e+01))
  (bind _splinebp (Variables|Default|GetSplineBP))
  (bind _floatingpawnmovement (Variables|Default|GetFloatingPawnMovement))
  (bind _paperflipbook (Variables|Default|GetPaperFlipbook))
  (bind _spline (Variables|/Game/BP_FigureEightSpline.BP_FigureEightSpline_C|GetSpline _splinebp))
  (if (Variables|Default|GetisHappy)
    (if (Math|Vector|Equal(Vector) (Transformation|GetActorLocation) (Spline|GetLocationatDistanceAlongSpline _spline (Math|Float|%(Float) (stale _result) (Spline|GetSplineLength _spline)) "World") 0.001)
      (bind _result (Math|Float|IncrementFloat (Variables|Default|GetSpline%20Dist))
        (:%20%20
          (Transformation|SetWorldLocation (Variables|Default|GetDummyRoot) (Spline|GetLocationatDistanceAlongSpline _spline (Math|Float|%(Float) _result (Spline|GetSplineLength _spline)) "World") false false)))
      (else
        (Transformation|SetActorRotation (Math|Rotator|FindLookatRotation _returnvalue (Spline|GetLocationatDistanceAlongSpline _spline (Math|Float|%(Float) _result (Spline|GetSplineLength _spline)) "World")))
        (Class|PawnMovementComponent|AddInputVector _floatingpawnmovement (- (Spline|GetLocationatDistanceAlongSpline _spline (Math|Float|%(Float) _result (Spline|GetSplineLength _spline)) "World") _returnvalue) false)
        (Sprite|SetFlipbook _paperflipbook "/Game/Source/Assets/Flipbooks/bat_flying.bat_flying")))
    (elif (Math|Vector|Equal(Vector) _returnvalue _returnvalue_2 0.1)
      (Sprite|SetFlipbook _paperflipbook "/Game/Source/Assets/Flipbooks/bat_hanging_Flipbook.bat_hanging_Flipbook")
      (else
        (Transformation|SetActorRotation (Math|Rotator|FindLookatRotation _returnvalue _returnvalue_2) true)
        (Class|PawnMovementComponent|AddInputVector _floatingpawnmovement (- _returnvalue_2 _returnvalue) false)))))

(event Collision|EventActorBeginOverlap
  (params (OtherActor :type Actor%20Object%20Reference))
  (Utilities|Casting|CastToBP_Wave OtherActor)
  (CallFunction|IncrementBatState))

(fn ConstructionScript)

(fn SetBatState
  (if (> (Utilities|Time|GetGameTimeinSeconds (Game|GetGameState)) 5.0)
    (Utilities|FlowControl|Sequence
      (:then_0
        (if (Math|Float|InRange(Float) (Variables|Default|GetBatHappinessThreshold) 0.0 0.1)
          (Variables|Default|SetBatSatus "NewEnumerator5")
          (Variables|Default|SetisHappy false)))
      (:then_1
        (if (Math|Float|InRange(Float) (Variables|Default|GetBatHappinessThreshold) 0.1 0.4 false)
          (Variables|Default|SetBatSatus "NewEnumerator4")))
      (:then_2
        (if (Math|Float|InRange(Float) (Variables|Default|GetBatHappinessThreshold) 0.4 0.6 false)
          (Variables|Default|SetBatSatus "NewEnumerator3")
          (Variables|Default|SetisHappy true)))
      (:then_3
        (if (Math|Float|InRange(Float) (Variables|Default|GetBatHappinessThreshold) 0.6 0.9 false)
          (Variables|Default|SetBatSatus "NewEnumerator2")
          (Variables|Default|SetisHappy true)))
      (:then_4
        (if (Math|Float|InRange(Float) (Variables|Default|GetBatHappinessThreshold) 0.9 1.0 false)
          (Variables|Default|SetBatSatus "NewEnumerator1")
          (Variables|Default|SetisHappy true))))
    (else
      (Variables|Default|SetBatSatus "NewEnumerator0"))))

(fn GetBatState
  (return (Variables|Default|GetBatSatus)))

(fn DecrementBatState
  (if (> (Variables|Default|GetBatHappinessThreshold) 0.01)
    (Variables|Default|SetBatHappinessThreshold (- (Variables|Default|GetBatHappinessThreshold) 0.01))))

(fn IncrementBatState
  (Variables|Default|SetBatHappinessThreshold (+ (Variables|Default|GetBatHappinessThreshold) 0.02)))