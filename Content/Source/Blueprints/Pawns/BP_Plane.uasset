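; BP_Plane is a pawn that flies continuously along world +X and scores work when it meets matching waves.
; FloatingPawnMovement gets constant input each tick, while a looping timer periodically snaps the plane back to a fixed start position.
; When its box collider overlaps a BP_Wave whose plane material equals AcceptedMaterial, it calls IncreaseWork on the first player's BP_PlayerState.
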(event OnComponentBeginOverlap(BoxCollider)
  (params (OverlappedComponent :type Primitive%20Component%20Object%20Reference) (OtherActor :type Actor%20Object%20Reference) (OtherComp :type Primitive%20Component%20Object%20Reference) (OtherBodyIndex :type Integer) (bFromSweep :type Boolean) (SweepResult :type Hit%20Result%20Structure%20%28by%20ref%29))
  (Utilities|IsValid OtherActor
    (:Is%20Valid
      (bind _asbp_wave (Utilities|Casting|CastToBP_Wave OtherActor))
      (bind _asbp_player_state (Utilities|Casting|CastToBP_PlayerState (Utilities|Array|Get(acopy) (Variables|/Script/Engine.GameStateBase|GetPlayerArray (Game|GetGameState)))))
      (if (== (Rendering|Material|GetMaterial (Variables|/Game/Source/Blueprints/Projectiles/BP_Wave.BP_Wave_C|GetPlane _asbp_wave) 0) (Variables|Default|GetAcceptedMaterial))
        (Default|IncreaseWork _asbp_player_state)))))

(event EventBeginPlay
  (Utilities|Time|SetTimerbyFunctionName 0 "PlaneMove" 35.0 true))

(event EventTick
  (params (DeltaSeconds :type Float%20%28single-precision%29))
  (Class|PawnMovementComponent|AddInputVector (Variables|Default|GetFloatingPawnMovement) "1.000000, 0, 0" false))

(fn ConstructionScript)

(fn PlaneMove
  (Transformation|SetActorLocation "-3000.000000,0.000000,610.000000" false false))