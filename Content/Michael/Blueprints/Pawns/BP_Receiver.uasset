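; BP_Receiver is a wandering pawn that catches waves and credits work to the player when their material matches.
; A looping timer picks a random X/Z direction, which Tick feeds into FloatingPawnMovement.
; On overlap with a Wave-tagged BP_Wave, it compares the plane's material to AcceptedMaterial, prints the result and destroys the wave.
; Matches call IncreaseWork on the first BP_PlayerState in the GameState's PlayerArray.
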(event Custom|IncreaseWork
  (bind _asbp_game_state (Utilities|Casting|CastToBP_GameState (Game|GetGameState)))
  (bind _asbp_player_state (Utilities|Casting|CastToBP_PlayerState (Utilities|Array|Get(acopy) (Variables|/Script/Engine.GameStateBase|GetPlayerArray _asbp_game_state))))
  (Default|IncreaseWork _asbp_player_state))

(event Collision|EventActorBeginOverlap
  (params (OtherActor :type Actor%20Object%20Reference))
  ;[0 0 0] On collision with wave print string to see if valid color
  (Utilities|IsValid OtherActor
    (:Is%20Valid
      (if (Actor|ActorHasTag OtherActor "Wave")
        (bind _asbp_wave (Utilities|Casting|CastToBP_Wave OtherActor))
        (if (== (Rendering|Material|GetMaterial (Variables|/Game/Michael/Blueprints/Projectiles/BP_Wave.BP_Wave_C|GetPlane _asbp_wave) 0) (Variables|Default|GetAcceptedMaterial))
          (Development|PrintString "GOOD!")
          (CallFunction|IncreaseWork)
          (else
            (Development|PrintString "BAD!")))
        (Actor|DestroyActor OtherActor)))))

(event EventBeginPlay
  (Utilities|Time|SetTimerbyFunctionName 0 "ChangeDirection" (Variables|Default|GetTimer) true))

(event EventTick
  (params (DeltaSeconds :type Float%20%28single-precision%29))
  ;[0 0 0] Update movement vector every frame
  (Class|PawnMovementComponent|AddInputVector (Variables|Default|GetFloatingPawnMovement) (Variables|Default|GetMovementVector) false))

(event Collision|EventHit
  (params (MyComp :type Primitive%20Component%20Object%20Reference) (Other :type Actor%20Object%20Reference) (OtherComp :type Primitive%20Component%20Object%20Reference) (bSelfMoved :type Boolean) (HitLocation :type Vector :default "0, 0, 0") (HitNormal :type Vector :default "0, 0, 0") (NormalImpulse :type Vector :default "0, 0, 0") (Hit :type Hit%20Result%20Structure%20%28by%20ref%29)))

(fn ConstructionScript)

(fn ChangeDirection
  (Variables|Default|SetMovementVector (Math|Vector|MakeVector (Math|Random|RandomFloatinRange -1.0 1.0) 0.0 (Math|Random|RandomFloatinRange -1.0 1.0))))