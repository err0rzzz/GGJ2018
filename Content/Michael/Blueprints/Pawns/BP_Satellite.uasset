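; BP_Satellite is a satellite that loops along a spline and credits the player with work when a wave overlaps it.
; BeginPlay snaps its DummyRoot to the start of the referenced SplineBP's spline.
; Each Tick advances it a fixed, frame-rate-dependent distance, wrapped by spline length.
; Overlapping a BP_Wave calls IncreaseWork on the first BP_PlayerState in the GameState's PlayerArray.
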(event Custom|ArcMovement
  (bind _splinebp (Variables|Default|GetSplineBP))
  (bind _spline (Variables|/Game/Michael/Blueprints/Actors/BP_ArcSpline.BP_ArcSpline_C|GetSpline _splinebp))
  (bind _output_get (Variables|Default|SetSplineDist (+ (Variables|Default|GetSplineDist) 1.0)))
  (Transformation|SetWorldLocation (Variables|Default|GetDummyRoot) (Spline|GetLocationatDistanceAlongSpline _spline (Math|Float|%(Float) _output_get (Spline|GetSplineLength _spline)) "World") false false))

(event Collision|EventActorBeginOverlap
  (params (OtherActor :type Actor%20Object%20Reference))
  (Utilities|Casting|CastToBP_Wave OtherActor)
  (bind _asbp_player_state (Utilities|Casting|CastToBP_PlayerState (Utilities|Array|Get(acopy) (Variables|/Script/Engine.GameStateBase|GetPlayerArray (Game|GetGameState)))))
  (Default|IncreaseWork _asbp_player_state))

(event EventTick
  (params (DeltaSeconds :type Float%20%28single-precision%29))
  (CallFunction|ArcMovement))

(event EventBeginPlay
  (Variables|Default|SetSplineDist 0.0)
  (Transformation|SetWorldLocation (Variables|Default|GetDummyRoot) (Spline|GetLocationatDistanceAlongSpline (Variables|/Game/Michael/Blueprints/Actors/BP_ArcSpline.BP_ArcSpline_C|GetSpline (Variables|Default|GetSplineBP)) (Variables|Default|GetSplineDist) "World") false false))

(fn ConstructionScript)